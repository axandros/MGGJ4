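; Base fighter Blueprint for a fighting game that controls which way each fighter actor faces.
; BeginPlay caches the FightingGameMode_BP, which supplies the opponent reference, and Tick calls UpdateRotation.
; Player one rotates the whole actor to look at player two, while any other fighter is held at zero rotation.
; Disconnected mesh-only look-at rotation nodes for both players remain in the function and never run.
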(event `self.ReceiveBeginPlay`
  (bind _asfighting_game_mode_bp (cast `/Game/FightingGameMode_BP` (`GameplayStatics.GetGameMode`)))
  (set `self.Fighting Game Mode` _asfighting_game_mode_bp))

(event `self.ReceiveTick`
  (params (DeltaSeconds :type "Float (single-precision)"))
  (`self.UpdateRotation`))

(fn `UpdateRotation`
  (if (`self._isPlayerOne`)
    (`self.K2_SetActorRotation` (`KismetMathLibrary.FindLookAtRotation` (`self.K2_GetActorLocation`) (`self.K2_GetActorLocation` (`FightingGameMode.PlayerTwo` (`self.Fighting Game Mode`)))))
    (else
      (`self.K2_SetActorRotation` (struct)))))

(fn `UserConstructionScript`)