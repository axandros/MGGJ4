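; Game mode for the fighting mode that sets up the match on BeginPlay.
; It finds the FightingModeCamera, spawns a fighter at each PlayerStart based on its tag, then adds the fighting interface widget.
; P1 spawns a SailorSenshiFighter possessed by controller 0 and viewed through that camera; other tags spawn a generic MGGJ4Character.
; P2 spawns a KyotoCat, but its possession and view setup for controller 1 never run.
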(event `self.ReceiveBeginPlay`
  (bind _outactors (`GameplayStatics.GetAllActorsOfClass` "/Game/FightingModeCamera.FightingModeCamera_C"))
  (for _array_element _outactors
    (set `self.MainView` _array_element)
    (break))
  (bind _outactors_2 (`GameplayStatics.GetAllActorsOfClass` "/Script/Engine.PlayerStart"))
  (for _array_element_2 _outactors_2
    (`self.SpawnPlayer` _array_element_2))
  (bind _returnvalue (`|CreateWidget` "/Game/GUI/UI_fightingInterface.UI_fightingInterface_C" (`GameplayStatics.GetPlayerController` 0)))
  (`UserWidget.AddToViewport` _returnvalue 0))

(fn `SpawnPlayer`
  (params (PlayerStart :type "PlayerStart Object Reference"))
  (bind _returnvalue (`self.GetTransform` PlayerStart))
  (bind _returnvalue_2 (`GameplayStatics.GetPlayerController` 0))
  (switch `name` (`PlayerStart.PlayerStartTag` PlayerStart)
    (:`Default`
      (`|SpawnActorFromClass` "/Script/MGGJ4.MGGJ4Character" _returnvalue "Undefined" "OverrideRootScale" PlayerStart null))
    (:`P1`
      (bind _returnvalue_3 (`|SpawnActorFromClass` "/Game/Fighters/SailorSenshi/SailorSenshiFighter.SailorSenshiFighter_C" _returnvalue "Undefined" "OverrideRootScale" PlayerStart null))
      (bind _output_get (set `self.PlayerOne` _returnvalue_3))
      (`AbstractFighter.SetAsPlayerOne` _output_get true)
      (`Controller.Possess` _returnvalue_2 _output_get)
      (`PlayerController.SetViewTargetWithBlend` _returnvalue_2 (`self.MainView`) 0.0 "VTBlend_Linear" 0.0 false))
    (:`P2`
      (bind _returnvalue_4 (`|SpawnActorFromClass` "/Game/Fighters/KyotoCat/KyotoCat.KyotoCat_C" _returnvalue "Undefined" "OverrideRootScale" PlayerStart null))
      (bind _output_get_2 (set `self.PlayerTwo` _returnvalue_4)))))

(fn `UserConstructionScript`)